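; Game mode Blueprint that runs a countdown and signals death on the player's HUD when time runs out.
; BeginPlay starts a looping one-second timer that calls Time, which decrements TimeCounter.
; Once the counter passes zero, Time adds the second back and calls SetDie on HUDVillage through FirstPersonHUD.
; The timer is never cleared, so that call repeats each second after expiry.
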(event EventBeginPlay
  (Utilities|Time|SetTimerbyFunctionName 0 "Time" 1.0 true))

(fn ConstructionScript)

(fn Time
  (bind _output_get (Variables|Default|SetTimeCounter (- (Variables|Default|GetTimeCounter) 1.0)))
  (if (<= _output_get -1.0)
    (Variables|Default|SetTimeCounter (+ (Variables|Default|GetTimeCounter) 1.0))
    (bind _asfirst_person_hud (Utilities|Casting|CastToFirstPersonHUD (HUD|GetHUD (Game|GetPlayerController 0))))
    (Default|SetDie (Variables|/Game/FirstPersonBP/Blueprints/FirstPersonHUD.FirstPersonHUD_C|GetHUD%20Village _asfirst_person_hud))))