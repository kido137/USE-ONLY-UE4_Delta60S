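; BP_SplintMove is a Level 2 actor that shuttles a cube back and forth along a spline.
; On BeginPlay a timeline plays or reverses according to the IsMoveR flag, which flips each time the timeline finishes, looping the motion endlessly.
; Each update scales the timeline value by the spline's length and sets the cube's world location and rotation from that point on the spline.
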(event EventBeginPlay
  (bind _spline (Variables|Default|GetSpline))
  (if (Variables|Default|GetIsMoveR) :!label _label
    (bind _value (Timeline|타임라인_0 Play)
      (:Update
        (Transformation|SetWorldLocationAndRotation (Variables|Default|GetCube) (Spline|GetLocationatDistanceAlongSpline _spline (* _value (Spline|GetSplineLength _spline)) "World") (Spline|GetRotationatDistanceAlongSpline _spline (* _value (Spline|GetSplineLength _spline)) "World") false false))
      (:Finished
        (Variables|Default|SetIsMoveR (not (Variables|Default|GetIsMoveR)))
        (goto _label)))
    (else
      (Timeline|타임라인_0 Reverse))))

(fn ConstructionScript)