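; BP_LCollision is a Level 2 actor that moves its Cube component around a square loop in the local X-Z plane.
; Each Tick switches on the IsMoveRight direction enum (right, up, left, down) and offsets the cube by a fixed step without sweep.
; When the relative location passes that edge's bound, the enum advances to the next direction, so speed depends on frame rate.
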(event EventTick
  (params (DeltaSeconds :type Float%20%28single-precision%29))
  (bind _cube (Variables|Default|GetCube))
  (bind _cube_2 (Variables|Default|GetCube))
  (bind _cube_3 (Variables|Default|GetCube))
  (bind _cube_4 (Variables|Default|GetCube))
  (switch Utilities|FlowControl|Switch|SwitchonEN_Move_Tybe (Variables|Default|GetIsMoveRight)
    (:NewEnumerator0
      (Transformation|AddLocalOffset _cube_4 "5.000000, 0, 0" false false)
      (if (> (.x (Variables|/Script/Engine.SceneComponent|GetRelativeLocation _cube_4)) 2e+02)
        (Variables|Default|SetIsMoveRight "NewEnumerator1")))
    (:NewEnumerator1
      (Transformation|AddLocalOffset _cube_2 "0.000000,0.000000,5.000000" false false)
      (if (> (.z (Variables|/Script/Engine.SceneComponent|GetRelativeLocation _cube_2)) 2e+02)
        (Variables|Default|SetIsMoveRight "NewEnumerator2")))
    (:NewEnumerator2
      (Transformation|AddLocalOffset _cube "-5.000000,0.000000,0.000000" false false)
      (if (< (.x (Variables|/Script/Engine.SceneComponent|GetRelativeLocation _cube)) 0.0)
        (Variables|Default|SetIsMoveRight "NewEnumerator3")))
    (:NewEnumerator3
      (Transformation|AddLocalOffset _cube_3 "-0.000000,0.000000,-5.000000" false false)
      (if (< (.z (Variables|/Script/Engine.SceneComponent|GetRelativeLocation _cube_3)) 0.0)
        (Variables|Default|SetIsMoveRight "NewEnumerator0")))))

(fn ConstructionScript)