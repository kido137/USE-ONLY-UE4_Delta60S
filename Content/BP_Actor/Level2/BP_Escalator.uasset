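; BP_Escalator is a Level 2 actor that builds an escalator from spawned floor pieces along a spline.
; On BeginPlay it divides the spline length by SpawnGap and spawns BP_EscalatorFloor actors at the spline component's transform.
; Each floor receives the spline, a distance offset in SpawnGap increments and a shared Speed, leaving placement and any movement to the floor actor.
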(event EventBeginPlay
  (for _index (range 0 (Math|Float|Floor (/ (Spline|GetSplineLength (Variables|Default|GetSpline)) (Variables|Default|GetSpawnGap))))
    (Game|SpawnActorfromClass "/Game/BP_Actor/Level2/BP_EscalatorFloor.BP_EscalatorFloor_C" (Transformation|GetWorldTransform (Variables|Default|GetSpline)) "Undefined" 0 (Variables|Default|GetSpline) (* _index (Variables|Default|GetSpawnGap)) (Variables|Default|GetSpeed) 0)))

(fn ConstructionScript)