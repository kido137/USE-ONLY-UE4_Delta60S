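; Level 2 escalator floor actor that loops a Cube along the Escalator spline and teleports Leefa to a fixed location on hit or overlap.
; A fast looping timer runs MoveOnSpline, advancing Distance by Speed and matching the Cube's location and rotation to the spline.
; At the spline's end, SleepTime disables collision, then ResetPosition snaps the Cube to the start, restores collision and restarts movement.
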(event OnComponentHit(Cube)
  (params (HitComponent :type Primitive%20Component%20Object%20Reference) (OtherActor :type Actor%20Object%20Reference) (OtherComp :type Primitive%20Component%20Object%20Reference) (NormalImpulse :type Vector :default "0, 0, 0") (Hit :type Hit%20Result%20Structure%20%28by%20ref%29))
  (bind _asleefa (Utilities|Casting|CastToLeefa OtherActor))
  (Transformation|SetActorLocation _asleefa "1000.000000, 0,200.000000" false false))

(event OnComponentBeginOverlap(Cube)
  (params (OverlappedComponent :type Primitive%20Component%20Object%20Reference) (OtherActor :type Actor%20Object%20Reference) (OtherComp :type Primitive%20Component%20Object%20Reference) (OtherBodyIndex :type Integer) (bFromSweep :type Boolean) (SweepResult :type Hit%20Result%20Structure%20%28by%20ref%29))
  (bind _asleefa (Utilities|Casting|CastToLeefa OtherActor))
  (Transformation|SetActorLocation _asleefa "1000.000000, 0,200.000000" false false))

(event EventBeginPlay
  (Utilities|Time|SetTimerbyFunctionName 0 "MoveOnSpline" 0.01 true))

(fn ConstructionScript)

(fn MoveonSpline
  (bind _escalator (Variables|Default|GetEscalator))
  (Variables|Default|SetDistance (+ (Variables|Default|GetDistance) (Variables|Default|GetSpeed)))
  (Transformation|SetWorldLocationAndRotation (Variables|Default|GetCube) (Spline|GetLocationatDistanceAlongSpline _escalator (Variables|Default|GetDistance) "World") (Spline|GetRotationatDistanceAlongSpline _escalator (Variables|Default|GetDistance) "World") false false)
  (if (>= (Variables|Default|GetDistance) (Spline|GetSplineLength (Variables|Default|GetEscalator)))
    (Utilities|Time|ClearTimerbyFunctionName 0 "MoveOnSpline")
    (CallFunction|SleepTime)))

(fn ResetPosition
  (bind _escalator (Variables|Default|GetEscalator))
  (bind _cube (Variables|Default|GetCube))
  (bind _output_get (Variables|Default|SetDistance 0.0))
  (Transformation|SetWorldLocationAndRotation _cube (Spline|GetLocationatDistanceAlongSpline _escalator _output_get "World") (Spline|GetRotationatDistanceAlongSpline _escalator _output_get "World") false false)
  (Collision|SetCollisionEnabled _cube "QueryAndPhysics")
  (Utilities|Time|SetTimerbyFunctionName 0 "MoveOnSpline" 0.01 true))

(fn SleepTime
  (Collision|SetCollisionEnabled (Variables|Default|GetCube) "NoCollision")
  (Utilities|Time|SetTimerbyFunctionName 0 "ResetPosition" 0.1))