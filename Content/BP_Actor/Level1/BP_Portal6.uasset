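; BP_Portal6 is a portal that stays hidden and non-colliding until all BP_Target actors in the level are hidden, then sends play to the MENU level on overlap.
; On BeginPlay it gathers every target and binds an event to each.
; Auto-generated handler functions call CheckAllHide to test the targets' sphere visibility and toggle the portal Sphere's visibility and collision to match.
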(event OnComponentBeginOverlap(Sphere)
  (params (OverlappedComponent :type Primitive%20Component%20Object%20Reference) (OtherActor :type Actor%20Object%20Reference) (OtherComp :type Primitive%20Component%20Object%20Reference) (OtherBodyIndex :type Integer) (bFromSweep :type Boolean) (SweepResult :type Hit%20Result%20Structure%20%28by%20ref%29))
  (Game|OpenLevel(byName) "MENU"))

(event EventBeginPlay
  (Rendering|SetVisibility (Variables|Default|GetSphere) false false)
  (Collision|SetCollisionEnabled (Variables|Default|GetSphere) "NoCollision")
  (bind _outactors (Actor|GetAllActorsOfClass "/Game/BP_Actor/Level1/BP_Target.BP_Target_C"))
  (Variables|Default|SetALL%20Target _outactors)
  (for _array_element _outactors
    (EventDispatchers|BindEventtoTarget _array_element (EventDispatchers|CreateEvent :!event BPPortalAutoGenFunc1))))

(event EventTick
  (params (DeltaSeconds :type Float%20%28single-precision%29)))

(fn ConstructionScript)

(fn CheckAllHide
  (for _array_element (Variables|Default|GetALL%20Target)
    (if (Rendering|IsVisible (Variables|/Game/BP_Actor/Level1/BP_Target.BP_Target_C|GetBP_Sphere _array_element))
      (return false)))
  (return true))

(fn BPPortalAutoGenFunc
  (params (OverlappedActor :type Actor%20Object%20Reference) (OtherActor :type Actor%20Object%20Reference))
  (bind _sphere (Variables|Default|GetSphere))
  (bind _newparam (CallFunction|CheckAllHide))
  (Rendering|SetVisibility (Variables|Default|GetSphere) _newparam false)
  (if _newparam
    (Collision|SetCollisionEnabled _sphere "QueryAndPhysics")
    (else
      (Collision|SetCollisionEnabled _sphere "NoCollision"))))

(fn BPPortalAutoGenFunc1
  (bind _sphere (Variables|Default|GetSphere))
  (bind _newparam (CallFunction|CheckAllHide))
  (Rendering|SetVisibility (Variables|Default|GetSphere) _newparam false)
  (if _newparam
    (Collision|SetCollisionEnabled _sphere "QueryAndPhysics")
    (else
      (Collision|SetCollisionEnabled _sphere "NoCollision"))))