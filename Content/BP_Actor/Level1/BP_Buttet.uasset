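; BP_Buttet is a physics-driven projectile actor that launches forward when spawned.
; BeginPlay applies a forward impulse to its Sphere and starts a short timer that calls Life Time to destroy the actor.
; Overlap and hit handlers only cast to Leefa, with no resulting effect.
; Per-frame offset movement and mesh knockback on Leefa are left as disconnected nodes.
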(event OnComponentBeginOverlap(Sphere)
  (params (OverlappedComponent :type Primitive%20Component%20Object%20Reference) (OtherActor :type Actor%20Object%20Reference) (OtherComp :type Primitive%20Component%20Object%20Reference) (OtherBodyIndex :type Integer) (bFromSweep :type Boolean) (SweepResult :type Hit%20Result%20Structure%20%28by%20ref%29))
  (Utilities|Casting|CastToLeefa OtherActor))

(event OnComponentHit(Sphere)
  (params (HitComponent :type Primitive%20Component%20Object%20Reference) (OtherActor :type Actor%20Object%20Reference) (OtherComp :type Primitive%20Component%20Object%20Reference) (NormalImpulse :type Vector :default "0, 0, 0") (Hit :type Hit%20Result%20Structure%20%28by%20ref%29))
  (bind _asleefa (Utilities|Casting|CastToLeefa OtherActor)))

(event EventBeginPlay
  (Physics|AddImpulse (Variables|Default|GetSphere) (* (Transformation|GetActorForwardVector) 1e+03) "None" false)
  (Utilities|Time|SetTimerbyFunctionName 0 "Life Time" 5.0))

(event EventTick
  (params (DeltaSeconds :type Float%20%28single-precision%29)))

(fn ConstructionScript)

(fn LifeTime
  (Actor|DestroyActor))