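; BP_Move_Cube is a Level 4 actor that moves a cube back and forth along a spline.
; A timeline track, scaled by spline length, sets the cube's world location and rotation from the spline each update.
; BeginPlay starts the timeline forward or in reverse based on the Move flag.
; On finish, Move flips and the branch runs again, creating a continuous ping-pong loop.
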(event EventBeginPlay
  (bind _spline (Variables|Default|GetSpline))
  (if (Variables|Default|GetMove) :!label _label
    (bind _새_트랙_0 (Timeline|타임라인_0 Play)
      (:Update
        (Transformation|SetWorldLocationAndRotation (Variables|Default|GetCube) (Spline|GetLocationatDistanceAlongSpline _spline (* _새_트랙_0 (Spline|GetSplineLength _spline)) "World") (Spline|GetRotationatDistanceAlongSpline _spline (* _새_트랙_0 (Spline|GetSplineLength _spline)) "World") false false))
      (:Finished
        (Variables|Default|SetMove (not (Variables|Default|GetMove)))
        (goto _label)))
    (else
      (Timeline|타임라인_0 Reverse))))

(fn ConstructionScript)