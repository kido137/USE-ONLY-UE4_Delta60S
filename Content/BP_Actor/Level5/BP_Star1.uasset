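; BP_Star1 is a homing projectile that chases the first player's pawn and explodes on contact.
; It faces the pawn on BeginPlay, then each Tick lerps slightly toward it and moves forward by a fixed, unswept offset that ignores delta time.
; Sphere hit or overlap spawns an explosion, plays a sound and destroys the actor.
; Overlap also launches Leefa, using a look-at from Leefa's location to itself, so the direction ignores the star.
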(event OnComponentHit(Sphere)
  (params (HitComponent :type Primitive%20Component%20Object%20Reference) (OtherActor :type Actor%20Object%20Reference) (OtherComp :type Primitive%20Component%20Object%20Reference) (NormalImpulse :type Vector :default "0, 0, 0") (Hit :type Hit%20Result%20Structure%20%28by%20ref%29))
  (Effects|SpawnEmitteratLocation "/Game/StarterContent/Particles/P_Explosion.P_Explosion" (Transformation|GetActorLocation) (Transformation|GetActorRotation) "1.000000,1.000000,1.000000" true "AutoRelease")
  (Audio|PlaySound2D "/Engine/VREditor/Sounds/UI/Foliage_Placed.Foliage_Placed" 1.0 1.0 0.0 0 0)
  (Actor|DestroyActor))

(event OnComponentBeginOverlap(Sphere)
  (params (OverlappedComponent :type Primitive%20Component%20Object%20Reference) (OtherActor :type Actor%20Object%20Reference) (OtherComp :type Primitive%20Component%20Object%20Reference) (OtherBodyIndex :type Integer) (bFromSweep :type Boolean) (SweepResult :type Hit%20Result%20Structure%20%28by%20ref%29))
  (Effects|SpawnEmitteratLocation "/Game/StarterContent/Particles/P_Explosion.P_Explosion" (Transformation|GetActorLocation) (Transformation|GetActorRotation) "1.000000,1.000000,1.000000" true "AutoRelease")
  (Audio|PlaySound2D "/Engine/VREditor/Sounds/UI/Foliage_Placed.Foliage_Placed" 1.0 1.0 0.0 0 0)
  (Actor|DestroyActor)
  (bind _asleefa (Utilities|Casting|CastToLeefa OtherActor))
  (Character|LaunchCharacter _asleefa (* (Math|Vector|GetForwardVector (Math|Rotator|FindLookatRotation (Transformation|GetActorLocation _asleefa) (Transformation|GetActorLocation _asleefa))) -1e+04) true true))

(event EventBeginPlay
  (Variables|Default|SetTargActor (Game|Player|GetPlayerPawn 0))
  (Transformation|SetActorRotation (Math|Rotator|FindLookatRotation (Transformation|GetActorLocation) (Transformation|GetActorLocation (Variables|Default|GetTargActor)))))

(event EventTick
  (params (DeltaSeconds :type Float%20%28single-precision%29))
  (bind _targactor (Variables|Default|GetTargActor))
  (Utilities|IsValid _targactor
    (:Is%20Valid
      (Transformation|SetActorRotation (Math|Rotator|Lerp(Rotator) (Transformation|GetActorRotation) (Math|Rotator|FindLookatRotation (Transformation|GetActorLocation) (Transformation|GetActorLocation _targactor)) 0.02 true))
      (Transformation|AddActorWorldOffset (* (Transformation|GetActorForwardVector) 3e+01)))))

(fn ConstructionScript)